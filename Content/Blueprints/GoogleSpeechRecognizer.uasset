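; Speech recognizer Blueprint that bridges captured microphone or audio input to a Google speech recognition service on localhost via HTTP POST requests.
; SetGrammar uploads a GRXML file's bytes with an enabled state and stores the grammar name, while SetLanguage and SetSpeechHandler store language and handler.
; OnSpeechInputCaptured posts raw samples as audio/l16 with rate, channels, grammar and language, then passes the response to the handler's OnSpeechRecognizedMessage.
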(event EventOnSpeechInputCaptured
  (params (Samples :type Array%20of%20Bytes) (Channels :type Integer) (SamplesPerSecond :type Integer))
  (Utilities|FlowControl|Sequence
    (:then_0
      (Variables|Default|SetRequest_0 (Class|VaRestRequestJSON|ConstructRequestExt "POST" "binary")))
    (:then_1
      (Class|VaRestRequestJSON|SetBinaryContentType (Variables|Default|GetRequest_0) (Utilities|String|ToString(Text) (Utilities|Text|FormatText "audio/l16; rate={SamplesPerSecond}; channels={Channels}" (Utilities|Text|ToText(Integer) SamplesPerSecond false) (Utilities|Text|ToText(Integer) Channels false)))))
    (:then_2
      (Class|VaRestRequestJSON|SetBinaryRequestContent (Variables|Default|GetRequest_0) Samples)
      (bind _result (Class|VaRestRequestJSON|ApplyURL (Variables|Default|GetRequest_0) (Utilities|String|ToString(Text) (Utilities|Text|FormatText "http://localhost:8081/google-recognize?grammar={Grammar}&lang={lang}" (Utilities|Text|ToText(String) (Variables|Default|GetGrammar)) (Utilities|Text|ToText(String) (Variables|Default|GetLang))))))
      (Class|ISpeechRecognizer|OnSpeechRecognized(Message) (Utilities|ToObject(Interface) (Variables|Default|GetSpeechRecognizer)) _result))))

(event EventSetGrammar
  (params (Grxml%20File :type String) (Enabled :type Boolean))
  (Utilities|FlowControl|Sequence
    (:then_0
      (Variables|Default|SetRequest_1 (Class|VaRestRequestJSON|ConstructRequestExt "POST" "binary")))
    (:then_1
      (Class|VaRestRequestJSON|SetBinaryRequestContent (Variables|Default|GetRequest_1) (.ResultBytes (Class|FileUtilsBPLibrary|ReadFile Grxml%20File)))
      (Class|VaRestRequestJSON|ApplyURL (Variables|Default|GetRequest_1) (Utilities|String|ToString(Text) (Utilities|Text|FormatText "http://localhost:8081/google-set-grammar?grammar={Grammar}&state={State}" (Utilities|Text|ToText(String) Grxml%20File) (Utilities|Text|ToText(Boolean) Enabled))))
      (Development|PrintString "Apply URL returned"))
    (:then_2
      (Variables|Default|SetGrammar Grxml%20File))))

(event EventSetLanguage
  (params (Language :type String))
  (Variables|Default|SetLang Language))

(event EventSetSpeechHandler
  (params (SpeechRecognizer :type I%20Speech%20Recognizer%20Interface))
  (Variables|Default|SetSpeechRecognizer SpeechRecognizer))

(fn ConstructionScript)