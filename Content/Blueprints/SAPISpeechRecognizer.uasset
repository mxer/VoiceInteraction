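; Blueprint wrapper around SAPI speech recognition that passes recognized speech to a registered handler.
; Grammar events load a GRXML file with an enabled flag, while language changes select UK or US English, defaulting to US, then pause and resume recognition.
; Recognized speech text is decoded as JSON and forwarded to the stored SpeechRecognizer handler.
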(event EventSetLanguage
  (params (Language :type String))
  (if (Utilities|Enum|Equal(Enum) Language "en-UK")
    (Class|SAPIPluginBlueprintLibrary|SetLanguage "Lang_EnglishUK")
    (else
      (Class|SAPIPluginBlueprintLibrary|SetLanguage "Lang_EnglishUS")))
  (Class|SAPIPluginBlueprintLibrary|PauseSpeechRecognition)
  (Class|SAPIPluginBlueprintLibrary|ResumeSpeechRecognition))

(event EventSetGrammar
  (params (Grxml%20File :type String) (Enabled :type Boolean))
  (Class|SAPIPluginBlueprintLibrary|SetGrammar Grxml%20File Enabled))

(event EventOnSpeechRecognized
  (params (SpeechText :type String))
  (bind _output_get (Variables|Default|SetJSON (Class|VaRestJsonObject|ConstructJsonObject)))
  (Class|VaRestJsonObject|DecodeJson _output_get SpeechText)
  (Default|OnSpeechRecognized (Variables|Default|GetSpeechRecognizer) _output_get))

(event EventSetSpeechHandler
  (params (SpeechRecognizer :type I%20Speech%20Recognizer%20Interface))
  (Variables|Default|SetSpeechRecognizer SpeechRecognizer))

(fn ConstructionScript)