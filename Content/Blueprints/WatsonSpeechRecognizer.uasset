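; Speech recognizer Blueprint that connects captured audio to IBM Watson speech recognition through a local HTTP service on port 8081.
; SetGrammar uploads a grammar file with its enabled state and stores its name, while SetLanguage stores the language used for recognition.
; Captured samples are posted as raw L16 audio with rate, channels, grammar and language.
; The JSON response goes to the registered speech handler and is printed.
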(event EventOnSpeechInputCaptured
  (params (Samples :type Array%20of%20Bytes) (Channels :type Integer) (SamplesPerSecond :type Integer))
  (Utilities|FlowControl|Sequence
    (:then_1
      (bind _output_get (Variables|Default|SetRequest (Class|VaRestRequestJSON|ConstructRequestExt "POST" "binary")))
      (Class|VaRestRequestJSON|SetBinaryContentType _output_get (Utilities|String|ToString(Text) (Utilities|Text|FormatText "audio/l16; rate={SamplesPerSecond}; channels={Channels}" (Utilities|Text|ToText(Integer) SamplesPerSecond false) (Utilities|Text|ToText(Integer) Channels false))))
      (Class|VaRestRequestJSON|SetBinaryRequestContent _output_get Samples)
      (bind _result (Class|VaRestRequestJSON|ApplyURL _output_get (Utilities|String|ToString(Text) (Utilities|Text|FormatText "http://localhost:8081/ibm-recognize?grammar={grammar}&lang={lang}" (Utilities|Text|ToText(String) (Variables|Default|GetGrammar)) (Utilities|Text|ToText(String) (Variables|Default|GetLang))))))
      (Default|OnSpeechRecognized (Variables|Default|GetSpeech%20Recognizer) _result)
      (Development|PrintString (Class|VaRestJsonObject|EncodeJson _result)))))

(event EventSetGrammar
  (params (Grxml%20File :type String) (Enabled :type Boolean))
  (Utilities|FlowControl|Sequence
    (:then_0
      (Variables|Default|SetRequest_1 (Class|VaRestRequestJSON|ConstructRequestExt "POST" "binary"))
      (Variables|Default|SetGrammar Grxml%20File))
    (:then_1
      (Class|VaRestRequestJSON|SetBinaryRequestContent (Variables|Default|GetRequest_1) (.ResultBytes (Class|FileUtilsBPLibrary|ReadFile Grxml%20File)))
      (Class|VaRestRequestJSON|ApplyURL (Variables|Default|GetRequest_1) (Utilities|String|ToString(Text) (Utilities|Text|FormatText "http://localhost:8081/ibm-set-grammar?grammar={Grammar}&state={State}" (Utilities|Text|ToText(String) Grxml%20File) (Utilities|Text|ToText(Boolean) Enabled)))))))

(event EventSetLanguage
  (params (Language :type String))
  (Variables|Default|SetLang Language))

(event EventSetSpeechHandler
  (params (SpeechRecognizer :type I%20Speech%20Recognizer%20Interface))
  (Variables|Default|SetSpeech%20Recognizer SpeechRecognizer))

(fn ConstructionScript)